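; BP_Elevator is an elevator actor that makes one round trip each time Interact activates it.
; Tick moves it along its up vector at Speed until it rises HeightAmount above its recorded start height.
; A Delay of WaitTime holds it at the top, then Tick lowers it to that height and resets the state flags.
; Disconnected timer and Timeline nodes remain unused.
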(event `self.ReceiveTick`
  (params (DeltaSeconds :type "Float (single-precision)"))
  (bind (_returnvalue_x _returnvalue_y _returnvalue_z) (`KismetMathLibrary.BreakVector` (`self.K2_GetActorLocation`)))
  (bind (_returnvalue_x_2 _returnvalue_y_2 _returnvalue_z_2) (`KismetMathLibrary.BreakVector` (`self.K2_GetActorLocation`)))
  (bind (_returnvalue_x_3 _returnvalue_y_3 _returnvalue_z_3) (`KismetMathLibrary.BreakVector` (`self.K2_GetActorLocation`)))
  (if (`self.isActivated`)
    (if (`self.CanMove`)
      (if (`self.isInitialNotSet`)
        (set `self.InitialHeight` _returnvalue_z)
        (set `self.isInitialNotSet` false))
      (`self.K2_SetActorLocation` (+ (`self.K2_GetActorLocation`) (* (`self.GetActorUpVector`) (* (`self.Speed`) (`GameplayStatics.GetWorldDeltaSeconds`)))))
      (if (>= _returnvalue_z_3 (+ (`self.HeightAmount`) (`self.InitialHeight`)))
        (set `self.CanMove` false)
        (`KismetSystemLibrary.Delay` (`self.WaitTime`))
        (set `self.timelinefinalizo` true))
      (elif (`self.timelinefinalizo`)
        (`self.K2_SetActorLocation` (+ (`self.K2_GetActorLocation`) (* (* (`self.GetActorUpVector`) (-1.0 -1.0 -1.0)) (* (`self.Speed`) (`GameplayStatics.GetWorldDeltaSeconds`)))))
        (if (<= _returnvalue_z_2 (`self.InitialHeight`))
          (set `self.isActivated` false)
          (set `self.isInitialNotSet` false)
          (set `self.Wait` 0.0)
          (set `self.BoolMaloFucha` false)
          (set `self.timelinefinalizo` false)
          (set `self.CanMove` true))))))

(fn `Interact`
  (set `self.isActivated` true)
  (`KismetSystemLibrary.PrintString` "Se activo Elevator"))

(fn `UserConstructionScript`)