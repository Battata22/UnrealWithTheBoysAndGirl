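; Player controller that hooks up the possessed pawn's events, toggles the mouse cursor and hosts the save/load menu.
; On possess, it gets BP_HUD_New and binds delegates to the pawn's damage component and, for BP_Spyro, coin collection.
; BeginPlay creates a collapsed save/load widget and binds its save click.
; BindSaveEvent passes a slot to BP_GS, the game state, to save the game.
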(event `self.ReceivePossess`
  (params (PossessedPawn :type "Pawn Object Reference"))
  (bind _returnvalue (`self.GetComponentByClass` PossessedPawn "/Game/TODO/Blueprint/BP_DamageableComponent.BP_DamageableComponent_C"))
  (`/Engine/EditorBlueprintResources/StandardMacros.IsValid` _returnvalue
    (:`Is Valid`
      (bind _asbp_hud_new (cast `/Game/TODO/Blueprint/Menu/BP_HUD_New` (`self.GetHUD`)))
      (add `/Game/TODO/Blueprint/BP_DamageableComponent.OnDamage` _returnvalue (`|CreateDelegate` _asbp_hud_new :!event `DisplayNewLife`))
      (bind _asbp_spyro (cast `/Game/TODO/Blueprint/BP_Spyro` PossessedPawn))
      (add `/Game/TODO/Blueprint/BP_Spyro.OnCoinCollected` _asbp_spyro (`|CreateDelegate` _asbp_hud_new :!event `DisplayNewCoinsAmount`)))))

(event `SetMouseOff`
  (set `self.bShowMouseCursor` false))

(event `SetMouseOn`
  (set `self.bShowMouseCursor` true))

(event `self.ReceiveBeginPlay`
  (set `self.bShowMouseCursor` false)
  (`self.Create_WBP_SaveLoadMenu`)
  (cast `/Game/TODO/SaveGame/BP_GS` (`GameplayStatics.GetGameState`))
  (add `/Game/TODO/Menu/WBP_SaveLoadMenu.SaveClicked` (`self.WBP_SaveLoadMenuVar`) (`|CreateDelegate` :!event `BindSaveEvent`)))

(fn `BindSaveEvent`
  (params (SaveSlot :type Integer))
  (bind _asbp_gs (cast `/Game/TODO/SaveGame/BP_GS` (`GameplayStatics.GetGameState`)))
  (`/Game/TODO/SaveGame/BP_GS.SaveGameFile` _asbp_gs SaveSlot))

(fn `Create_WBP_SaveLoadMenu`
  (bind _returnvalue (`|CreateWidget` "/Game/TODO/Menu/WBP_SaveLoadMenu.WBP_SaveLoadMenu_C"))
  (`UserWidget.AddToViewport` _returnvalue 10)
  (bind _output_get (set `self.WBP_SaveLoadMenuVar` _returnvalue))
  (set `Widget.Visibility` "Collapsed" _output_get))

(fn `UserConstructionScript`)