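; BP_UniqueTagGenerator is a component that derives a numeric tag from its owner actor's transform.
; On BeginPlay it generates UniqueTag unless UseDefault is set or a non-zero tag already exists.
; GenerateTag combines location, rotation and scale into one absolute float, with CheckZero substituting a fixed non-zero value for zero inputs.
; The result is deterministic for a given transform, with no check for collisions between actors.
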(event `self.ReceiveBeginPlay`
  (if (`self.UseDefault`)
    _
    (elif (== (`self.UniqueTag`) 0.0)
      (bind _uniquetaggenerated (`self.GenerateTag`))
      (set `self.UniqueTag` _uniquetaggenerated))))

(fn `CheckZero`
  (params (Input :type "Float (double-precision)"))
  (returns (Output :type "Float (double-precision)"))
  (locals (EndOutput :type "Float (double-precision)"))
  (if (== Input 0.0)
    (set `local.EndOutput` 1.1)
    (else
      (set `local.EndOutput` Input)))
  (return (`local.EndOutput`)))

(fn `GenerateTag`
  (returns (UniqueTagGenerated :type "Float (double-precision)"))
  (locals (L_X :type "Float (double-precision)") (L_Y :type "Float (double-precision)") (L_Z :type "Float (double-precision)") (R_X :type "Float (double-precision)") (R_Y :type "Float (double-precision)") (R_Z :type "Float (double-precision)") (S_X :type "Float (double-precision)") (S_Y :type "Float (double-precision)") (S_Z :type "Float (double-precision)"))
  (bind _returnvalue (`Actor.GetTransform` (`self.GetOwner`)))
  (`|ExecutionSequence`
    (:`then_0`
      (bind _output (`self.CheckZero` (.x (.location _returnvalue))))
      (set `local.L_X` _output))
    (:`then_1`
      (bind _output_2 (`self.CheckZero` (.y (.location _returnvalue))))
      (set `local.L_Y` _output_2))
    (:`then_2`
      (bind _output_3 (`self.CheckZero` (.z (.location _returnvalue))))
      (set `local.L_Z` _output_3))
    (:`then_3`
      (bind _output_4 (`self.CheckZero` (.roll (.rotation _returnvalue))))
      (set `local.R_X` _output_4))
    (:`then_4`
      (bind _output_5 (`self.CheckZero` (.pitch (.rotation _returnvalue))))
      (set `local.R_Y` _output_5))
    (:`then_5`
      (bind _output_6 (`self.CheckZero` (.yaw (.rotation _returnvalue))))
      (set `local.R_Z` _output_6))
    (:`then_6`
      (bind _output_7 (`self.CheckZero` (.x (.scale _returnvalue))))
      (set `local.S_X` _output_7))
    (:`then_7`
      (bind _output_8 (`self.CheckZero` (.y (.scale _returnvalue))))
      (set `local.S_Y` _output_8))
    (:`then_8`
      (bind _output_9 (`self.CheckZero` (.z (.scale _returnvalue))))
      (set `local.S_Z` _output_9))
    (:`then_9`
      (return (`KismetMathLibrary.Abs` (+ (* (/ (* (`local.L_X`) (`local.S_Y`)) (`local.R_Z`)) (/ (* (`local.L_Y`) (`local.S_Z`)) (`local.R_X`)) (/ (* (`local.L_Z`) (`local.S_X`)) (`local.R_Y`))) (`local.L_Y`)))))))