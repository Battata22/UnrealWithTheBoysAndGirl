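; BP_FireArea is a hazard actor that deals damage on overlap, limited by a cooldown.
; Tick accumulates a Wait timer; when an overlap begins after Wait reaches Cooldown, it resets the timer and calls GetDamage on a BP_DamageableComponent.
; The overlap check also compares OtherActor to BP_DamageableComponent.
; Damage triggers only on overlap begin, so remaining inside the area does not repeat it.
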(event `self.ReceiveActorBeginOverlap`
  (params (OtherActor :type "Actor Object Reference"))
  (bind _returnvalue (`self.GetComponentByClass` "/Game/TODO/Blueprint/BP_DamageableComponent.BP_DamageableComponent_C"))
  (if (and (== OtherActor "/Game/TODO/Blueprint/BP_DamageableComponent.BP_DamageableComponent") (>= (stale `self.ReceiveTick` _output_get) (`self.Cooldown`)))
    (set `self.Wait` 0.0)
    (`/Engine/EditorBlueprintResources/StandardMacros.IsValid` _returnvalue
      (:`Is Valid`
        (`/Game/TODO/Blueprint/BP_DamageableComponent.GetDamage` _returnvalue (`self.Damage`))))))

(event `self.ReceiveTick`
  (params (DeltaSeconds :type "Float (single-precision)"))
  (bind _output_get (set `self.Wait` (+ (`GameplayStatics.GetWorldDeltaSeconds`) (`self.Wait`)))))

(fn `UserConstructionScript`)