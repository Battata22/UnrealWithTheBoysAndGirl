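; BP_LootChest is a loot chest that drops a heal and a coin when its PlayerContact function is called.
; It spawns BP_Heal and BP_Coin above itself, offset to opposite sides along Y.
; It then records its BPUniqueTagGenerator tag as a destroyed chest in BP_GI.
; Finally it teleports far out of the level instead of being destroyed, as the DestroyActor node is left unconnected.
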(fn `AddTagToGameInstance`
  (bind _asbp_gi (cast `/Game/TODO/SaveGame/BP_GI` (`GameplayStatics.GetGameInstance`)))
  (`/Game/TODO/SaveGame/BP_GI.AddDestroyedChest` _asbp_gi (`KismetStringLibrary.Conv_DoubleToString` (`/Game/TODO/Blueprint/BP_UniqueTagGenerator.UniqueTag` (`self.BP_UniqueTagGenerator`)))))

(fn `PlayerContact`
  (bind _returnvalue (`self.GetTransform`))
  (bind _returnvalue_2 (`self.GetTransform`))
  (`|ExecutionSequence`
    (:`then_0`
      (`|SpawnActorFromClass` "/Game/TODO/Blueprint/BP_Heal.BP_Heal_C" (`KismetMathLibrary.MakeTransform` (`KismetMathLibrary.MakeVector` (.x (.location _returnvalue)) (+ (.y (.location _returnvalue)) 75.0) (+ (.z (.location _returnvalue)) 250.0))) "Undefined" "MultiplyWithRoot" null null))
    (:`then_1`
      (`|SpawnActorFromClass` "/Game/TODO/Blueprint/BP_Coin.BP_Coin_C" (`KismetMathLibrary.MakeTransform` (`KismetMathLibrary.MakeVector` (.x (.location _returnvalue_2)) (+ (.y (.location _returnvalue_2)) -75.0) (+ (.z (.location _returnvalue_2)) 250.0))) "Undefined" "MultiplyWithRoot" null null)
      (`self.AddTagToGameInstance`)
      (`self.K2_SetActorLocation` (12121212.0 12121212.0 12121212.0)))))

(fn `UserConstructionScript`)