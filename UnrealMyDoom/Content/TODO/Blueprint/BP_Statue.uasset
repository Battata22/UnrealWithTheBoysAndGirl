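; BP_Statue is a save point that opens the save menu.
; On BeginPlay it caches the BP_GI game instance, which holds the shared save menu widget and the player controller.
; OpenMenu signals that the save menu is open, makes that widget visible and enables the mouse on BPPC_New.
; Its own controller lookup and menu-spawning functions are disconnected.
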(event `self.ReceiveBeginPlay`
  (bind _asbp_gi (cast `/Game/TODO/SaveGame/BP_GI` (`GameplayStatics.GetGameInstance`)))
  (set `self.GameInstanteVar` _asbp_gi))

(event `self.ReceiveEndPlay`
  (params (EndPlayReason :type "EEndPlayReason Enum" :default "Destroyed")))

(fn `GetPlayerController`)

(fn `Open Menu`
  (`self.SaveMenuOpen` true)
  (set `Widget.Visibility` "Visible" (`/Game/TODO/SaveGame/BP_GI.WBP_SaveMenu` (`self.GameInstanteVar`)))
  (bind _asbppc_new (cast `/Game/TODO/Blueprint/Menu/BPPC_New` (`/Game/TODO/SaveGame/BP_GI.PlayerController` (`self.GameInstanteVar`))))
  (`/Game/TODO/Blueprint/Menu/BPPC_New.SetMouseOn` _asbppc_new))

(fn `Spawn_WBP_SaveLoadMenu`)

(fn `UserConstructionScript`)