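; BP_IndianaRock is a boulder hazard that waits until the player enters its Collider, then chases them.
; An opened gate moves it a fixed step toward the player every Tick, horizontally only and not scaled by delta time.
; Sphere contact damages the player through BP_DamageableComponent.
; That hit, or LifeTime expiring after movement starts, calls IndianaRockDeath with the rock's unique tag and destroys it.
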(event `self.ReceiveTick`
  (params (DeltaSeconds :type "Float (single-precision)"))
  (bind _returnvalue (`self.K2_GetActorLocation`))
  (bind (_returnvalue_x _returnvalue_y) (`KismetMathLibrary.BreakVector` (+ (* (`KismetMathLibrary.GetDirectionUnitVector` (`self.K2_GetActorLocation`) (`self.K2_GetActorLocation` (`GameplayStatics.GetPlayerCharacter` 0))) 10.0) _returnvalue)))
  (`|ExecutionSequence`
    (:`then_0`
      (if (`self.SeMovioChuchaWea`)
        (bind _output_get (set `self.Wait` (+ (`GameplayStatics.GetWorldDeltaSeconds`) (`self.Wait`))))
        (if (>= _output_get (`self.LifeTime`))
          (`self.IndianaRockDeath` (`KismetStringLibrary.Conv_DoubleToString` (`/Game/TODO/Blueprint/BP_UniqueTagGenerator.UniqueTag` (`self.BP_UniqueTagGenerator`))))
          (`self.K2_DestroyActor`))))
    (:`then_1`
      (`/Engine/EditorBlueprintResources/StandardMacros.Gate` true :!label _label
        (:`Exit`
          (`self.K2_SetActorLocation` (`KismetMathLibrary.MakeVector` _returnvalue_x _returnvalue_y (.z _returnvalue)))
          (set `self.IsStill` false)
          (set `self.SeMovioChuchaWea` true))))))

(event `self.Collider.OnComponentBeginOverlap`
  (params (OverlappedComponent :type "PrimitiveComponent Object Reference") (OtherActor :type "Actor Object Reference") (OtherComp :type "PrimitiveComponent Object Reference") (OtherBodyIndex :type Integer) (bFromSweep :type Boolean) (SweepResult :type "HitResult Structure (by ref)"))
  (if (and (and (`PrimitiveComponent.IsOverlappingActor` (`self.Collider`) OtherActor) (`self.IsStill`)) (== OtherActor (`GameplayStatics.GetPlayerCharacter` 0)))
    (goto _label :!via `Open`)))

(event `self.Sphere.OnComponentBeginOverlap`
  (params (OverlappedComponent :type "PrimitiveComponent Object Reference") (OtherActor :type "Actor Object Reference") (OtherComp :type "PrimitiveComponent Object Reference") (OtherBodyIndex :type Integer) (bFromSweep :type Boolean) (SweepResult :type "HitResult Structure (by ref)"))
  (bind _returnvalue (`self.GetComponentByClass` OtherActor "/Game/TODO/Blueprint/BP_DamageableComponent.BP_DamageableComponent_C"))
  (if (== OtherActor (`GameplayStatics.GetPlayerCharacter` 0))
    (`/Engine/EditorBlueprintResources/StandardMacros.IsValid` _returnvalue
      (:`Is Valid`
        (`/Game/TODO/Blueprint/BP_DamageableComponent.GetDamage` _returnvalue (`self.Damage`))
        (`self.IndianaRockDeath` (`KismetStringLibrary.Conv_DoubleToString` (`/Game/TODO/Blueprint/BP_UniqueTagGenerator.UniqueTag` (`self.BP_UniqueTagGenerator`))))
        (`self.K2_DestroyActor`)))))

(fn `UserConstructionScript`)