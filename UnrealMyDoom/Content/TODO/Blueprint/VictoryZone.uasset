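; VictoryZone is a trigger actor that shows the victory screen when any actor begins overlapping it.
; The overlap clears all widgets, adds WBP_Victoria to the viewport and casts the player controller to BPPC_New to turn the mouse on.
; A boolean guard, named for the defeat screen having appeared, is set on first trigger so the sequence does not repeat.
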(event `self.ReceiveActorBeginOverlap`
  (params (OtherActor :type "Actor Object Reference"))
  (if (not (`self.YaSalioLaPantallaDeDerrotaSignoDeInterrogacion`))
    (`WidgetLayoutLibrary.RemoveAllWidgets`)
    (bind _returnvalue (`|CreateWidget` "/Game/TODO/Menu/WBP_Victoria.WBP_Victoria_C"))
    (`UserWidget.AddToViewport` _returnvalue 0)
    (set `self.YaSalioLaPantallaDeDerrotaSignoDeInterrogacion` true)
    (bind _returnvalue_2 (`InputDeviceLibrary.GetPlayerControllerFromPlatformUser` (`PlayerController.GetPlatformUserId` (`GameplayStatics.GetPlayerController` 0))))
    (bind _asbppc_new (cast `/Game/TODO/Blueprint/Menu/BPPC_New` _returnvalue_2))
    (`/Game/TODO/Blueprint/Menu/BPPC_New.SetMouseOn` _asbppc_new)))

(fn `UserConstructionScript`)