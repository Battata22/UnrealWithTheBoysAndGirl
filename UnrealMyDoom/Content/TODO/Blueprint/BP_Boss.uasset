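; Boss actor that advances through phases when hurt while vulnerable, driving its BPAI_Boss controller through Blackboard keys.
; BeginPlay sets the shoot interval on the Blackboard of the controller, which is found by class lookup and cached.
; Each hit increments Phase, resets the shot count and sets Destination to the BP_Coin whose UniqueTag matches the new phase.
; Player-sight perception logic exists but is disconnected.
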(event `self.ReceiveBeginPlay`
  (`self.SetShootInterval` 5))

(event `self.AIPerception.OnTargetPerceptionUpdated`
  (params (Actor :type "Actor Object Reference") (Stimulus :type "AIStimulus Structure")))

(fn `GetHurt_NextPhase`
  (if (`self.CanGetHurt`)
    (bind _bpai_boss (`self.GetMyAI`))
    (`self.SetNextPhase` (`AIBlueprintHelperLibrary.GetBlackboard` _bpai_boss))))

(fn `GetMyAI`
  (returns (BPAI_Boss :type "/Game/TODO/IA/Boss/BPAI_Boss Object Reference"))
  (`/Engine/EditorBlueprintResources/StandardMacros.IsValid` (`self.BPAI_Boss`)
    (:`Is Valid`
      _)
    (:`Is Not Valid`
      (bind _returnvalue (`GameplayStatics.GetActorOfClass` "/Game/TODO/IA/Boss/BPAI_Boss.BPAI_Boss_C"))
      (set `self.BPAI_Boss` _returnvalue)))
  (return (`self.BPAI_Boss`)))

(fn `ResetShoot`
  (params (BlackBoardRef :type "BlackboardComponent Object Reference"))
  (`BlackboardComponent.SetValueAsInt` BlackBoardRef (`KismetStringLibrary.Conv_StringToName` "ShootedAmount") 0))

(fn `Set New Destination`
  (bind _phase (`self.Phase`))
  (bind _outactors (`GameplayStatics.GetAllActorsOfClass` "/Game/TODO/Blueprint/BP_Coin.BP_Coin_C"))
  (for _array_element _outactors
    (if (== (`/Game/TODO/Blueprint/BP_UniqueTagGenerator.UniqueTag` (`self.GetComponentByClass` _array_element "/Game/TODO/Blueprint/BP_UniqueTagGenerator.BP_UniqueTagGenerator_C")) _phase)
      (`KismetSystemLibrary.PrintString` (`KismetStringLibrary.Conv_IntToString` _phase))
      (bind _returnvalue_location (`KismetMathLibrary.BreakTransform` (`self.GetTransform` _array_element)))
      (`BlackboardComponent.SetValueAsVector` (`AIBlueprintHelperLibrary.GetBlackboard` (`self.BPAI_Boss`)) (`KismetStringLibrary.Conv_StringToName` "Destination") _returnvalue_location))))

(fn `SetNextPhase`
  (params (BlackBoardRef :type "BlackboardComponent Object Reference"))
  (bind _returnvalue (`KismetStringLibrary.Conv_StringToName` "Phase"))
  (bind _returnvalue_2 (+ (`BlackboardComponent.GetValueAsInt` BlackBoardRef _returnvalue) 1))
  (set `self.Phase` _returnvalue_2)
  (`BlackboardComponent.SetValueAsInt` BlackBoardRef _returnvalue _returnvalue_2)
  (`self.ResetShoot` (`AIBlueprintHelperLibrary.GetBlackboard` (`self.BPAI_Boss`)))
  (`self.Set New Destination`))

(fn `SetShootInterval`
  (params (NewInterval :type Integer))
  (bind _bpai_boss (`self.GetMyAI`))
  (`BlackboardComponent.SetValueAsInt` (`AIBlueprintHelperLibrary.GetBlackboard` _bpai_boss) (`KismetStringLibrary.Conv_StringToName` "ShootInterval") NewInterval))

(fn `UserConstructionScript`)