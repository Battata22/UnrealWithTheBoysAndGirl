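; PuertaFinal is a final door that slides up when G is pressed or Abrir is called.
; Both set IsMoving, and Tick then records the starting height once and moves the actor along its up vector at Speed, scaled by delta time.
; Movement stops for good once it has risen HeightAmount.
; A timed wait-and-descend sequence sits unconnected in Abrir, so the door never closes.
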(event `Key|G`
  (params (Key :type "Key Structure"))
  (:`Pressed`
    (set `self.IsMoving` true)))

(event `self.ReceiveTick`
  (params (DeltaSeconds :type "Float (single-precision)"))
  (bind (_returnvalue_x _returnvalue_y _returnvalue_z) (`KismetMathLibrary.BreakVector` (`self.K2_GetActorLocation`)))
  (bind (_returnvalue_x_2 _returnvalue_y_2 _returnvalue_z_2) (`KismetMathLibrary.BreakVector` (`self.K2_GetActorLocation`)))
  (if (`self.IsMoving`)
    (if (`self.CanMove`)
      (if (`self.IsinitialSet`)
        (set `self.InitialHeight` _returnvalue_z)
        (set `self.IsinitialSet` false))
      (`self.K2_SetActorLocation` (+ (`self.K2_GetActorLocation`) (* (`self.GetActorUpVector`) (* (`self.Speed`) (`GameplayStatics.GetWorldDeltaSeconds`)))))
      (if (>= _returnvalue_z_2 (+ (`self.HeightAmount`) (`self.InitialHeight`)))
        (set `self.CanMove` false)))))

(fn `Abrir`
  (set `self.IsMoving` true))

(fn `UserConstructionScript`)