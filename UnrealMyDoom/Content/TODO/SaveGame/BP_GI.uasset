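; Game Instance that holds the game state for saving and controls the save and load menus.
; Setters record player stats, difficulty, timer, level and unique tags of destroyed coins, Indianas, chests and eggs, which GiveAllInfo returns together.
; Menu functions call open/close events, toggle visibility and mouse mode, and lazily cache widgets from the player controller.
; The load menu also works under BPPC_Menu, falling back when BPPC_New is absent.
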(event `self.ReceiveInit`)

(fn `AddDestroyedChest`
  (params (DestroyedChestTag :type String))
  (`KismetArrayLibrary.Array_AddUnique` (`self.DestroyedChestTags`) DestroyedChestTag))

(fn `AddDestroyedCoins`
  (params (CoinCollectedTag :type String))
  (`KismetArrayLibrary.Array_AddUnique` (`self.DestroyedCoinsTags`) CoinCollectedTag))

(fn `AddDestroyedEggs`
  (params (DestroyedEggTag :type String))
  (`KismetArrayLibrary.Array_AddUnique` (`self.DestroyedEggsTags`) DestroyedEggTag))

(fn `AddDestroyedIndianas`
  (params (CoinCollectedTag :type String))
  (`KismetArrayLibrary.Array_AddUnique` (`self.DestroyedIndianaTags`) CoinCollectedTag))

(fn `Close Load Menu`
  (`self.CloseMenu` false)
  (`Widget.SetVisibility` (`self.WBP_LoadMenu`) "Collapsed")
  (bind _asbppc_new (cast `/Game/TODO/Blueprint/Menu/BPPC_New` (`GameplayStatics.GetPlayerController` 0)))
  (`/Game/TODO/Blueprint/Menu/BPPC_New.SetMouseOff` _asbppc_new))

(fn `Close Save Menu`
  (`self.CloseMenu` false)
  (`Widget.SetVisibility` (`self.WBP_SaveMenu`) "Collapsed")
  (bind _asbppc_new (cast `/Game/TODO/Blueprint/Menu/BPPC_New` (`GameplayStatics.GetPlayerController` 0)))
  (`/Game/TODO/Blueprint/Menu/BPPC_New.SetMouseOff` _asbppc_new))

(fn `GiveAllInfo`
  (returns (PlayerPos :type "Vector Structure") (PlayerLife :type Integer) (PlayerCoinsCollectedAmount :type Integer) (RemaningTime :type "Float (double-precision)") (ActualLevel :type String) (Difficulty :type Integer) (DestroyedIndianaTags :type "Array of String") (DestroyedCoinsTags :type "Array of String") (DestroyedChestTags :type "Array of String") (DestroyedEggsTags :type "Array of String"))
  (return (`self.PlayerPos`) (`self.PlayerLife`) (`self.PlayerCoinsCollectedAmount`) (`self.RemaningTime`) (`self.ActualLevel`) (`self.Difficulty`) (`self.DestroyedIndianaTags`) (`self.DestroyedCoinsTags`) (`self.DestroyedChestTags`) (`self.DestroyedEggsTags`)))

(fn `OpenLoadMenu`
  (`self.SetWBP_LoadMenu`)
  (if (`|EnumEquality` (`Widget.Visibility` (`self.WBP_LoadMenu`)) "Collapsed")
    (`self.OpenMenu` false)
    (set `Widget.Visibility` "Visible" (`self.WBP_LoadMenu`))
    (bind _bppc_new (`self.SetPlayerController`))
    (`/Engine/EditorBlueprintResources/StandardMacros.IsValid` _bppc_new
      (:`Is Valid`
        (`/Game/TODO/Blueprint/Menu/BPPC_New.SetMouseOn` _bppc_new)))
    (else
      (`self.Close Load Menu`))))

(fn `OpenSaveMenu`
  (`self.OpenMenu` true)
  (bind _wbp_saveloadmenu (`self.SetWBP_SaveMenu`))
  (set `Widget.Visibility` "Visible" _wbp_saveloadmenu)
  (bind _bppc_new (`self.SetPlayerController`))
  (`/Game/TODO/Blueprint/Menu/BPPC_New.SetMouseOn` _bppc_new))

(fn `Set Difficulty`
  (params (Difficulty :type Integer))
  (set `self.Difficulty` Difficulty))

(fn `Set Player Info`
  (params (LastPos :type "Vector Structure") (Life :type Integer) (CoinsCollected :type Integer))
  (set `self.PlayerPos` LastPos)
  (set `self.PlayerLife` Life)
  (set `self.PlayerCoinsCollectedAmount` CoinsCollected))

(fn `SetLevelString`
  (bind _returnvalue (`GameplayStatics.GetCurrentLevelName` true))
  (set `self.ActualLevel` _returnvalue))

(fn `SetPlayerController`
  (returns (BPPC_New :type "/Game/TODO/Blueprint/Menu/BPPC_New Object Reference") (BPPC_Menu :type "/Game/TODO/Blueprint/Menu/BPPC_Menu Object Reference"))
  (bind _returnvalue (`GameplayStatics.GetPlayerController` 0))
  (`/Engine/EditorBlueprintResources/StandardMacros.IsValid` (`self.PlayerController`)
    (:`Is Valid`
      _)
    (:`Is Not Valid`
      (bind _asbppc_new (cast `/Game/TODO/Blueprint/Menu/BPPC_New` _returnvalue)
        (:`then`
          (set `self.PlayerController` _asbppc_new))
        (:`CastFailed`
          (bind _asbppc_menu (cast `/Game/TODO/Blueprint/Menu/BPPC_Menu` _returnvalue))))))
  (return (`self.PlayerController`) _asbppc_menu))

(fn `SetRemaningTimer`
  (params (RemaningTime :type "Float (double-precision)"))
  (set `self.RemaningTime` RemaningTime))

(fn `SetWBP_LoadMenu`
  (returns (WBP_LoadMenu :type "/Game/TODO/Menu/WBP_LoadMenu Object Reference"))
  (`/Engine/EditorBlueprintResources/StandardMacros.IsValid` (`self.WBP_LoadMenu`)
    (:`Is Valid`
      _)
    (:`Is Not Valid`
      (bind (_bppc_new _bppc_menu) (`self.SetPlayerController`))
      (`/Engine/EditorBlueprintResources/StandardMacros.IsValid` _bppc_new
        (:`Is Valid`
          (set `self.WBP_LoadMenu` (`/Game/TODO/Blueprint/Menu/BPPC_New.WBP_LoadMenuVar` _bppc_new)))
        (:`Is Not Valid`
          (set `self.WBP_LoadMenu` (`/Game/TODO/Blueprint/Menu/BPPC_Menu.WBP_LoadMenuVar` _bppc_menu))))))
  (return (`self.WBP_LoadMenu`)))

(fn `SetWBP_SaveMenu`
  (returns (WBP_SaveLoadMenu :type "/Game/TODO/Menu/WBP_SaveMenu Object Reference"))
  (`/Engine/EditorBlueprintResources/StandardMacros.IsValid` (`self.WBP_SaveMenu`)
    (:`Is Valid`
      _)
    (:`Is Not Valid`
      (bind _bppc_new (`self.SetPlayerController`))
      (set `self.WBP_SaveMenu` (`/Game/TODO/Blueprint/Menu/BPPC_New.WBP_SaveMenuVar` _bppc_new))))
  (return (`self.WBP_SaveMenu`)))