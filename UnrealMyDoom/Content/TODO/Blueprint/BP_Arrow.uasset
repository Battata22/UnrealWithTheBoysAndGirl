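; Arrow projectile actor that damages the third-person player character on contact.
; Sir stores the flight direction and rotation, and Tick moves the arrow along that direction without sweep, scaled by Speed, SpeedAdjust and delta time.
; Tick also reapplies the stored rotation with yaw and roll swapped.
; Overlapping the player calls GetDamaged and destroys the arrow; other overlaps are ignored.
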(event `self.ReceiveTick`
  (params (DeltaSeconds :type "Float (single-precision)"))
  (bind (_rot_roll _rot_pitch _rot_yaw) (`KismetMathLibrary.BreakRotator` (`self.rot`)))
  (`self.K2_SetActorLocation` (+ (`self.K2_GetActorLocation`) (* (`self.Dir`) (* (* (`self.Speed`) (`GameplayStatics.GetWorldDeltaSeconds`)) (`self.SpeedAdjust`)))))
  (`self.K2_SetActorRotation` (`KismetMathLibrary.MakeRotator` _rot_yaw _rot_pitch _rot_roll)))

(event `self.ReceiveBeginPlay`)

(event `self.ReceiveActorBeginOverlap`
  (params (OtherActor :type "Actor Object Reference"))
  (if (== OtherActor "/Game/ThirdPerson/Blueprints/BP_ThirdPersonCharacter.BP_ThirdPersonCharacter_C")
    (bind _asbp_third_person_character (cast `/Game/ThirdPerson/Blueprints/BP_ThirdPersonCharacter` OtherActor))
    (`/Game/ThirdPerson/Blueprints/BP_ThirdPersonCharacter.Get Damaged` _asbp_third_person_character (`self.Damage`))
    (`self.K2_DestroyActor`)))

(fn `sir`
  (params (dir :type "Vector Structure") (rot :type "Rotator Structure"))
  (set `self.Dir` dir)
  (set `self.rot` rot))

(fn `UserConstructionScript`)