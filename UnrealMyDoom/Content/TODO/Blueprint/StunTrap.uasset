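; StunTrap is a one-shot trap actor that immobilizes BP_Spyro when it overlaps the trap.
; The first overlap sets an Active guard and clears any lifespan so the trap persists through the stun.
; The StunTime timeline calls StopMovement on every update, then resumes movement and destroys the trap when finished.
; StartBlink and StopBlink calls are present but unconnected.
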(event `self.ReceiveActorBeginOverlap`
  (params (OtherActor :type "Actor Object Reference"))
  (bind _asbp_spyro (cast `/Game/TODO/Blueprint/BP_Spyro` OtherActor))
  (if (not (`self.Active`))
    (set `self.Active` true)
    (`self.SetLifeSpan` 0.0)
    (`Timeline|Timeline` :`NewTime` (`self.StunTime`) :!via `PlayFromStart`
      (:`Update`
        (`/Game/TODO/Blueprint/BP_Spyro.Stop Movement` _asbp_spyro))
      (:`Finished`
        (`/Game/TODO/Blueprint/BP_Spyro.ResumeMovement` _asbp_spyro)
        (`self.K2_DestroyActor`)))))

(fn `UserConstructionScript`)