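; Player controller for the main menu that shows the cursor, puts up the menu widget and plays a 2D sound on BeginPlay.
; It also creates the load menu widget on a higher layer, collapsed, and keeps a reference to it.
; The open-menu input action delegates to the game instance's OpenLoadMenu, as does a separate OpenLoadMenu function.
; Leftover VSync debug and options-widget nodes are disconnected.
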(event `self.ReceiveBeginPlay`
  (set `self.bShowMouseCursor` true)
  (`self.Create_WBP_LoadMenu`)
  (bind _returnvalue (`|CreateWidget` "/Game/TODO/Menu/WBP_Menu.WBP_Menu_C"))
  (`UserWidget.AddToViewport` _returnvalue 0)
  (`GameplayStatics.PlaySound2D` "/Game/TODO/Sounds/Music/BE_Blue.BE_Blue" 1.0 1.0 0.0 null null))

(event `self.ReceiveTick`
  (params (DeltaSeconds :type "Float (single-precision)")))

(event `EnhancedInput|/Game/TODO/Inputs/IA_OpenMenu`
  (params (ActionValue :type Boolean) (ElapsedSeconds :type "Float (double-precision)") (TriggeredSeconds :type "Float (double-precision)") (InputAction :type "InputAction Object Reference" :default "/Game/TODO/Inputs/IA_OpenMenu.IA_OpenMenu"))
  (:`Completed`
    (bind _asbp_gi (cast `/Game/TODO/SaveGame/BP_GI` (`GameplayStatics.GetGameInstance`)))
    (`/Game/TODO/SaveGame/BP_GI.OpenLoadMenu` _asbp_gi)))

(event `Key|Z`
  (params (Key :type "Key Structure")))

(fn `Create_WBP_LoadMenu`
  (bind _returnvalue (`|CreateWidget` "/Game/TODO/Menu/WBP_LoadMenu.WBP_LoadMenu_C"))
  (`UserWidget.AddToViewport` _returnvalue 11)
  (bind _output_get (set `self.WBP_LoadMenuVar` _returnvalue))
  (set `Widget.Visibility` "Collapsed" _output_get))

(fn `Open Load Menu`
  (bind _asbp_gi (cast `/Game/TODO/SaveGame/BP_GI` (`GameplayStatics.GetGameInstance`)))
  (`/Game/TODO/SaveGame/BP_GI.OpenLoadMenu` _asbp_gi))

(fn `UserConstructionScript`)