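; BP_DamageableComponent is a health component that lets its owning actor take damage and die.
; It fills current HP to the maximum on BeginPlay, and GetDamage subtracts incoming damage with clamping, then broadcasts OnDamage.
; At zero HP it broadcasts OnDeath and destroys the owner.
; A debug print for damage to BP_Spyro remains in the graph but never runs.
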(event `self.ReceiveBeginPlay`
  (set `self.CurrentHP` (`self.MaxHP`)))

(fn `GetDamage`
  (params (RecivedDMG :type Integer :default 1))
  (bind _output_get (set `self.CurrentHP` (`KismetMathLibrary.Clamp` (- (`self.CurrentHP`) RecivedDMG) 0 (`self.MaxHP`))))
  (`self.OnDamage` RecivedDMG _output_get)
  (if (== _output_get 0)
    (`self.OnDeath`)
    (`Actor.K2_DestroyActor` (`self.GetOwner`))))