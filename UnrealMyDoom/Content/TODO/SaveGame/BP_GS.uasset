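; Save-game manager that stores and restores player, gameplay, enemy and destroyed-actor data in one BP_SG slot.
; Each save function loads or creates the save object through SaveTheSaveFile, updates it and writes the slot.
; On the HUD's cargo-UI event, it binds Indiana rock deaths, records their tags and restores player position and life.
; Saved rock tags matching recorded ones trigger DestroyActor on this manager itself, not the rocks.
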(event `self.ReceiveBeginPlay`
  (bind _asbp_hud_new (cast `/Game/TODO/Blueprint/Menu/BP_HUD_New` (`PlayerController.GetHUD` (`GameplayStatics.GetPlayerController` 0))))
  (add `/Game/TODO/Blueprint/Menu/BP_HUD_New.YaCargoUI` _asbp_hud_new (delegate `Startedx`)))

(event `Startedx`
  (`self.BindIndianas`)
  (bind _returnvalue (`GameplayStatics.DoesSaveGameExist` "SaveGameFile"))
  (if _returnvalue
    (bind _returnvalue_2 (`GameplayStatics.LoadGameFromSlot` "SaveGameFile"))
    (bind _asbp_sg (cast `/Game/TODO/SaveGame/BP_SG` _returnvalue_2))
    (set `self.BP_SGVar` _asbp_sg)
    (`|ExecutionSequence`
      (:`then_0`
        (`self.SetLocationStart`))
      (:`then_1`
        (`self.SetLifeStart`))
      (:`then_2`
        (`self.DestroyActorsInSave` _asbp_sg)))
    (else
      (`/Game/TODO/Blueprint/BP_DamageableComponent.SetLife` (`self.GetComponentByClass` (`GameplayStatics.GetPlayerPawn` 0) "/Game/TODO/Blueprint/BP_DamageableComponent.BP_DamageableComponent_C") 3))))

(fn `BindCoins`
  (bind _outactors (`GameplayStatics.GetAllActorsOfClass` "/Game/TODO/Blueprint/BP_IndianaRock.BP_IndianaRock_C"))
  (for _array_element _outactors
    (bind _asbp_indiana_rock (cast `/Game/TODO/Blueprint/BP_IndianaRock` _array_element))
    (add `/Game/TODO/Blueprint/BP_IndianaRock.IndianaRockDeath` _asbp_indiana_rock (`|CreateDelegate` :!event `SaveDestroyedActors`))
    (`KismetSystemLibrary.PrintString` "asdsa"))
  (return))

(fn `BindIndianas`
  (bind _outactors (`GameplayStatics.GetAllActorsOfClass` "/Game/TODO/Blueprint/BP_IndianaRock.BP_IndianaRock_C"))
  (for _array_element _outactors
    (bind _asbp_indiana_rock (cast `/Game/TODO/Blueprint/BP_IndianaRock` _array_element))
    (add `/Game/TODO/Blueprint/BP_IndianaRock.IndianaRockDeath` _asbp_indiana_rock (`|CreateDelegate` :!event `SaveDestroyedActors`))
    (`KismetArrayLibrary.Array_AddUnique` (`self.IndianaTags`) (`KismetStringLibrary.Conv_DoubleToString` (`/Game/TODO/Blueprint/BP_UniqueTagGenerator.UniqueTag` (`self.GetComponentByClass` _asbp_indiana_rock "/Game/TODO/Blueprint/BP_UniqueTagGenerator.BP_UniqueTagGenerator_C")))))
  (return))

(fn `DestroyActorsInSave`
  (params (SaveFile :type "/Game/TODO/SaveGame/BP_SG Object Reference"))
  (bind _destroyedindianarocks (`/Game/TODO/SaveGame/BP_SG.DestroyedIndianaRocks` SaveFile))
  (if (`KismetArrayLibrary.Array_IsEmpty` _destroyedindianarocks)
    (`KismetSystemLibrary.PrintString` "vacia")
    (else
      (for _array_element _destroyedindianarocks
        (if (`KismetArrayLibrary.Array_Contains` (`self.IndianaTags`) _array_element)
          (`self.K2_DestroyActor`))))))

(fn `SaveDestroyedActors`
  (params (DestroyedActor :type String))
  (bind (_bp_sg _slotnameo) (`self.SaveTheSaveFile` "SaveGameFile"))
  (`/Game/TODO/SaveGame/BP_SG.AddToDestrtoyedActors` _bp_sg DestroyedActor)
  (`GameplayStatics.SaveGameToSlot` _bp_sg _slotnameo))

(fn `SaveEnemiesStates`
  (params (EnemiyState :type "Actor Object Reference"))
  (bind (_bp_sg _slotnameo) (`self.SaveTheSaveFile` "SaveGameFile"))
  (`/Game/TODO/SaveGame/BP_SG.SetEnemiesState` _bp_sg EnemiyState)
  (`GameplayStatics.SaveGameToSlot` _bp_sg _slotnameo))

(fn `SaveGameplayInfo`
  (params (Level :type Integer) (RemaningTime :type "Float (double-precision)") (Difficulty :type Integer) (CoinsCollected :type Integer))
  (bind (_bp_sg _slotnameo) (`self.SaveTheSaveFile` "SaveGameFile"))
  (`/Game/TODO/SaveGame/BP_SG.SetGameplayInfo` _bp_sg Level RemaningTime Difficulty CoinsCollected)
  (`GameplayStatics.SaveGameToSlot` _bp_sg _slotnameo))

(fn `SavePlayerInfo`
  (params (LastPos :type "Vector Structure") (Life :type Integer))
  (bind (_bp_sg _slotnameo _exist) (`self.SaveTheSaveFile` "SaveGameFile"))
  (`/Game/TODO/SaveGame/BP_SG.SetPlayerInfo` _bp_sg LastPos Life)
  (`GameplayStatics.SaveGameToSlot` _bp_sg _slotnameo))

(fn `SaveTheSaveFile`
  (params (SlotName :type String))
  (returns (BP_SG :type "/Game/TODO/SaveGame/BP_SG Object Reference") (SlotNameO :type String) (Exist :type Boolean))
  (locals (SGOutput :type "/Game/TODO/SaveGame/BP_SG Object Reference") (BoolExist :type Boolean))
  (bind _returnvalue (`GameplayStatics.DoesSaveGameExist` SlotName))
  (if _returnvalue
    (bind _returnvalue_2 (`GameplayStatics.LoadGameFromSlot` SlotName))
    (bind _asbp_sg (cast `/Game/TODO/SaveGame/BP_SG` _returnvalue_2))
    (set `local.SGOutput` _asbp_sg)
    (set `local.BoolExist` true)
    (else
      (`KismetSystemLibrary.PrintString` "Hello")
      (bind _returnvalue_3 (`GameplayStatics.CreateSaveGameObject` "/Game/TODO/SaveGame/BP_SG.BP_SG_C"))
      (set `local.SGOutput` _returnvalue_3)
      (set `local.BoolExist` false)))
  (return (`local.SGOutput`) SlotName (`local.BoolExist`)))

(fn `SetLifeStart`
  (bind _playerlife (`/Game/TODO/SaveGame/BP_SG.PlayerLife` (`self.BP_SGVar`)))
  (if (== _playerlife 0)
    (`/Game/TODO/Blueprint/BP_DamageableComponent.SetLife` (`self.GetComponentByClass` (`GameplayStatics.GetPlayerPawn` 0) "/Game/TODO/Blueprint/BP_DamageableComponent.BP_DamageableComponent_C") 3)
    (else
      (`/Game/TODO/Blueprint/BP_DamageableComponent.SetLife` (`self.GetComponentByClass` (`GameplayStatics.GetPlayerPawn` 0) "/Game/TODO/Blueprint/BP_DamageableComponent.BP_DamageableComponent_C") _playerlife))))

(fn `SetLocationStart`
  (bind (_playerpos_x _playerpos_y _playerpos_z) (`KismetMathLibrary.BreakVector` (`/Game/TODO/SaveGame/BP_SG.PlayerPos` (`self.BP_SGVar`))))
  (if (not (>= _playerpos_z 100000.0))
    (`self.K2_SetActorLocation` (`GameplayStatics.GetPlayerPawn` 0) (`KismetMathLibrary.MakeVector` _playerpos_x _playerpos_y _playerpos_z) false false)
    (`KismetSystemLibrary.PrintString` (`KismetStringLibrary.Conv_VectorToString` (+ (`KismetMathLibrary.MakeVector` _playerpos_x _playerpos_y _playerpos_z) (`KismetMathLibrary.Vector_Zero`))))))

(fn `UserConstructionScript`)