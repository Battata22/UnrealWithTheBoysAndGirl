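; BP_Egg is a collectible egg pickup that reacts when Spyro overlaps its mesh.
; On overlap it plays the Coin sound, records its unique tag in the game instance's destroyed-egg list, and calls CollectCoin on Spyro with a zero argument.
; The tag comes from a BPUniqueTagGenerator, and the egg does not destroy itself in this graph.
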(event `self.EggMesh.OnComponentBeginOverlap`
  (params (OverlappedComponent :type "PrimitiveComponent Object Reference") (OtherActor :type "Actor Object Reference") (OtherComp :type "PrimitiveComponent Object Reference") (OtherBodyIndex :type Integer) (bFromSweep :type Boolean) (SweepResult :type "HitResult Structure (by ref)"))
  (bind _asbp_spyro (cast `/Game/TODO/Blueprint/BP_Spyro` OtherActor))
  (`GameplayStatics.PlaySoundAtLocation` "/Game/TODO/Sounds/SFX/coin.coin" (`self.K2_GetActorLocation`) (struct) 1.0 1.0 0.0 null null null null)
  (`self.AddTagToGameInstance`)
  (`/Game/TODO/Blueprint/BP_Spyro.CollectCoin` _asbp_spyro 0))

(fn `AddTagToGameInstance`
  (bind _asbp_gi (cast `/Game/TODO/SaveGame/BP_GI` (`GameplayStatics.GetGameInstance`)))
  (`/Game/TODO/SaveGame/BP_GI.AddDestroyedEggs` _asbp_gi (`KismetStringLibrary.Conv_DoubleToString` (`/Game/TODO/Blueprint/BP_UniqueTagGenerator.UniqueTag` (`self.BP_UniqueTagGenerator`)))))

(fn `UserConstructionScript`)