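; BP_FireBallBoss is a projectile, apparently the boss's fireball, that moves along a direction set through Sir, which also zeroes its rotation.
; Tick moves it manually without sweeping; overlapping an actor with BP_DamageableComponent plays a sound, deals damage and teleports the fireball far away instead of destroying it.
; LoadDataTable reads difficulty-specific speed and scale from DT_EnemyData, but its call in the event graph is disconnected.
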(event `self.ReceiveBeginPlay`)

(event `self.ReceiveTick`
  (params (DeltaSeconds :type "Float (single-precision)"))
  (bind (_rot_roll _rot_pitch _rot_yaw) (`KismetMathLibrary.BreakRotator` (`self.rot`)))
  (`self.K2_SetActorLocation` (+ (`self.K2_GetActorLocation`) (* (`self.Dir`) (* (* (`self.Speed`) (`GameplayStatics.GetWorldDeltaSeconds`)) (`self.SpeedAdjust`)))))
  (`self.K2_SetActorRotation` (`KismetMathLibrary.MakeRotator` _rot_yaw _rot_pitch _rot_roll)))

(event `self.ReceiveActorBeginOverlap`
  (params (OtherActor :type "Actor Object Reference"))
  (bind _returnvalue (`self.GetComponentByClass` OtherActor "/Game/TODO/Blueprint/BP_DamageableComponent.BP_DamageableComponent_C"))
  (`/Engine/EditorBlueprintResources/StandardMacros.IsValid` _returnvalue
    (:`Is Valid`
      (`GameplayStatics.PlaySoundAtLocation` "/Game/StarterContent/Audio/disparo.disparo" (`self.K2_GetActorLocation`) (struct) 1.0 1.0 0.0 null null null null)
      (`/Game/TODO/Blueprint/BP_DamageableComponent.GetDamage` _returnvalue (`self.Damage`))
      (`self.K2_SetActorLocation` (1111111.0 1111111.0 1111111.0) false true))
    (:`Is Not Valid`
      (cast `/Game/TODO/Blueprint/BP_SpawnerFlechas` OtherActor))))

(fn `Load Data Table`
  (locals (RowName :type String :default "Test"))
  (bind (_returnvalue_location _returnvalue_rotation) (`KismetMathLibrary.BreakTransform` (`self.GetTransform`)))
  (bind _rowname (`local.RowName`))
  (bind _rowname_2 (`local.RowName`))
  (bind _asbp_gi (cast `/Game/TODO/SaveGame/BP_GI` (`GameplayStatics.GetGameInstance`)))
  (if (== (`/Game/TODO/SaveGame/BP_GI.Difficulty` _asbp_gi) 1)
    (set `self.DataTable_Row_Name` _rowname_2)
    (set `self.RowNameToRead` (`KismetStringLibrary.Conv_StringToName` (`KismetStringLibrary.Concat_StrStr` _rowname_2 "1")))
    (else
      (set `self.DataTable_Row_Name` _rowname)
      (set `self.RowNameToRead` (`KismetStringLibrary.Conv_StringToName` (`KismetStringLibrary.Concat_StrStr` _rowname "2")))))
  (bind _returnvalue (`|GetDataTableRow` "/Game/TODO/Blueprint/DataTableClass/DT_EnemyData.DT_EnemyData" (`self.RowNameToRead`))
    (:`then`
      (bind (_scale _speed _speedadjust) (break `/Game/TODO/Blueprint/DataTableClass/FE_EnemyData` _returnvalue))
      (set `self.Speed` _speed)
      (set `self.SpeedAdjust` _speedadjust)
      (`self.K2_SetActorTransform` (`KismetMathLibrary.MakeTransform` _returnvalue_location _returnvalue_rotation (`KismetMathLibrary.Conv_DoubleToVector` _scale))))))

(fn `sir`
  (params (dir :type "Vector Structure"))
  (set `self.Dir` dir)
  (set `self.rot` (struct)))

(fn `UserConstructionScript`)