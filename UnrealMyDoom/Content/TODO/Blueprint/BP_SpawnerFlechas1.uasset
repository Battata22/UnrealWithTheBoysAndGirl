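; BP_SpawnerFlechas1 is a placed arrow spawner that periodically fires BP_Arrow actors.
; Tick feeds delta time into SpawnArrow, which accumulates it in Wait and resets the counter once it reaches Cooldown.
; Each arrow spawns at the spawner's location with a hardcoded rotation, then receives the spawner's forward vector and rotation through its Sir function.
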(event `self.ReceiveBeginPlay`)

(event `self.ReceiveTick`
  (params (DeltaSeconds :type "Float (single-precision)"))
  (`self.SpawnArrow` DeltaSeconds))

(fn `SpawnArrow`
  (params (DeltaTime :type "Float (double-precision)"))
  (bind _returnvalue_location (`KismetMathLibrary.BreakTransform` (`self.GetTransform`)))
  (bind _output_get (set `self.Wait` (+ DeltaTime (`self.Wait`))))
  (if (>= _output_get (`self.Cooldown`))
    (set `self.Wait` 0.0)
    (bind _returnvalue (`|SpawnActorFromClass` "/Game/TODO/Blueprint/BP_Arrow.BP_Arrow_C" (`KismetMathLibrary.MakeTransform` _returnvalue_location (struct :`Pitch` -90.0 :`Yaw` 180.0 :`Roll` 180.0)) "AdjustIfPossibleButAlwaysSpawn" "MultiplyWithRoot" null null))
    (`/Game/TODO/Blueprint/BP_Arrow.sir` _returnvalue (`self.GetActorForwardVector`) (`self.K2_GetActorRotation`))))

(fn `UserConstructionScript`)