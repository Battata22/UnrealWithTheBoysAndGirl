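; Ogre actor, prefixed OLD, that gets knocked back when rammed.
; GetDamaged starts a push unless one is active and prints a debug message.
; Tick moves the ogre horizontally away from player 0 by PushSpeed times a factor that decays linearly over about one second, then ends the push.
; The per-frame step is not scaled by delta time, so push distance depends on frame rate.
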(event `self.ReceiveTick`
  (params (DeltaSeconds :type "Float (single-precision)"))
  (bind _returnvalue (`self.K2_GetActorLocation`))
  (bind (_returnvalue_x _returnvalue_y) (`KismetMathLibrary.BreakVector` (+ (* (* (`KismetMathLibrary.GetDirectionUnitVector` (`self.K2_GetActorLocation` (`GameplayStatics.GetPlayerCharacter` 0)) (`self.K2_GetActorLocation`)) (`self.PushSpeed`)) (`self.SpeedOverTime`)) _returnvalue)))
  (if (`self.IsBeenPushed`)
    (`self.K2_SetActorLocation` (`KismetMathLibrary.MakeVector` _returnvalue_x _returnvalue_y (.z _returnvalue)))
    (bind _output_get (set `self.SpeedOverTime` (- (`self.SpeedOverTime`) (`GameplayStatics.GetWorldDeltaSeconds`))))
    (if (<= _output_get 0.0)
      (set `self.IsBeenPushed` false))
    (else
      (set `self.SpeedOverTime` 1.0))))

(fn `GetDamaged`
  (if (not (`self.IsBeenPushed`))
    (`KismetSystemLibrary.PrintString` (`KismetStringLibrary.Concat_StrStr` (`KismetSystemLibrary.GetObjectName` self) " Fue embestido") true true (struct :`R` 0.108014 :`G` 0.83 :`A` 1.0))
    (set `self.IsBeenPushed` true)))

(fn `UserConstructionScript`)